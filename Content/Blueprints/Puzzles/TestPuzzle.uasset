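; TestPuzzle is a puzzle Blueprint, apparently for testing, that assembles its parts and answerer from child actors.
; On BeginPlay it scans its ChildActorComponents and adds child actors that cast to PuzzlePart to the PuzzleParts array.
; It then casts the TestAnswerer component's child actor to PuzzleAnswerer and adds it to PuzzleAnswerers.
; The graph only registers these actors and holds no solving logic.
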(event `self.ReceiveBeginPlay`
  (for _array_element (`self.K2_GetComponentsByClass` "/Script/Engine.ChildActorComponent")
    (bind _aspuzzle_part (cast `PuzzlePart` (`ChildActorComponent.ChildActor` _array_element)))
    (`KismetArrayLibrary.Array_Add` (`self.PuzzleParts`) _aspuzzle_part))
  (bind _aspuzzle_answerer (cast `PuzzleAnswerer` (`ChildActorComponent.ChildActor` (`self.Test Answerer`))))
  (`KismetArrayLibrary.Array_Add` (`self.PuzzleAnswerers`) _aspuzzle_answerer))

(fn `UserConstructionScript`)