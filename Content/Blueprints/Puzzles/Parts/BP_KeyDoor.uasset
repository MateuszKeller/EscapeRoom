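; BP_KeyDoor is a puzzle door that opens when the player clicks it with the required item.
; On click, an item check decides whether to spawn a BP_Key, snap it to the mesh's KeyHole socket and instantly rotate the door mesh 90 degrees.
; A failed check shows a rejection message through the player character cached on BeginPlay.
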(event `self.ReceiveBeginPlay`
  (bind _asbp_player_character (cast `/Game/Blueprints/BP_PlayerCharacter` (`GameplayStatics.GetPlayerCharacter` 0)))
  (set `self.Player` _asbp_player_character))

(event `self.PuzzlePartMeshComponent.OnClicked`
  (params (TouchedComponent :type "PrimitiveComponent Object Reference") (ButtonPressed :type "Key Structure"))
  (bind _returnvalue (`ItemComponent.CheckUsedItem` (`self.Item`)))
  (if _returnvalue
    (bind _returnvalue_2 (`|SpawnActorFromClass` "/Game/Blueprints/Items/T/BP_Key.BP_Key_C" (`self.GetTransform`) "AlwaysSpawn" "OverrideRootScale" null null))
    (`self.K2_AttachToComponent` _returnvalue_2 (`self.PuzzlePartMeshComponent`) "KeyHole" "SnapToTarget" "SnapToTarget" "SnapToTarget" true)
    (`SceneComponent.K2_SetRelativeRotation` (`self.PuzzlePartMeshComponent`) (struct :`Yaw` -90.0) false false)
    (else
      (`/Game/Blueprints/BP_PlayerCharacter.Display Message` (`self.Player`) "You Picked The Wrong House Foul"))))

(fn `UserConstructionScript`)