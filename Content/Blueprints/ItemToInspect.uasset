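; Inspectable item actor that the player can examine and rotate with the mouse.
; Looking at it sends an "Inspect" prompt with the item name to the HUD, and interacting calls Inspect for that player.
; Its own input handlers yaw and pitch the root component from mouse movement while the right button is held, and call Drop on the Interact action.
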(event `self.OnLookAt`
  (params (Player :type "PlayerCharacter Object Reference"))
  (`/Game/Libraries/HUDFormatingLibrary.UpdateHUDMessage` Player "Inspect" (`self.ItemName`)))

(event `self.InteractWith`
  (params (Player :type "PlayerCharacter Object Reference"))
  (`self.Inspect` Player))

(event `Key|RightMouseButton`
  (params (Key :type "Key Structure"))
  (:`Pressed`
    (set `self.isRotating` true))
  (:`Released`
    (set `self.isRotating` false)))

(event `InputAxisKey|MouseX`
  (params (AxisValue :type "Float (single-precision)"))
  (if (`self.isRotating`)
    (`SceneComponent.K2_AddRelativeRotation` (`self.RootComponent`) (`KismetMathLibrary.MakeRotator` 0.0 0.0 (* AxisValue 3.0)) false false)))

(event `InputAxisKey|MouseY`
  (params (AxisValue :type "Float (single-precision)"))
  (if (`self.isRotating`)
    (`SceneComponent.K2_AddRelativeRotation` (`self.RootComponent`) (`KismetMathLibrary.MakeRotator` 0.0 (* AxisValue 3.0)) false false)))

(event `InputAction|Interact`
  (params (Key :type "Key Structure"))
  (:`Pressed`
    (`self.Drop`)))

(fn `UserConstructionScript`)