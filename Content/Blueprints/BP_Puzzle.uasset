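; Interactable puzzle actor that shows a "Solve Puzzle" prompt when looked at and switches the player into a puzzle view.
; Interacting pauses the player's tick, clears the HUD message and calls ChangeView; the Interact input restores tick and calls it again.
; Holding right mouse orbits the camera, with mouse X yawing the camera root and mouse Y pitching the spring arm.
; Clicking its Item hands it to the player through PickUp.
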(event `InputAction|Interact`
  (params (Key :type "Key Structure"))
  (:`Pressed`
    (`self.SetActorTickEnabled` (stale `self.InteractWith` Player) true)
    (`self.ChangeView`)))

(event `self.InteractWith`
  (params (Player :type "PlayerCharacter Object Reference"))
  (`self.SetActorTickEnabled` Player false)
  (bind _asbp_player_character (cast `/Game/Blueprints/BP_PlayerCharacter` Player))
  (`/Game/UI/HUD.UpdateMessage` (`/Game/Blueprints/BP_PlayerCharacter.HUD` _asbp_player_character) "")
  (`self.ChangeView`))

(event `self.OnLookAt`
  (params (Player :type "PlayerCharacter Object Reference"))
  (`/Game/Libraries/HUDFormatingLibrary.UpdateHUDMessage` Player "Solve" "Puzzle"))

(event `self.Item.OnClicked`
  (params (TouchedComponent :type "PrimitiveComponent Object Reference") (ButtonPressed :type "Key Structure"))
  (bind _asbp_player_character (cast `/Game/Blueprints/BP_PlayerCharacter` (`GameplayStatics.GetPlayerCharacter` 0)))
  (`ItemComponent.PickUp` (`self.Item`) _asbp_player_character))

(event `Key|RightMouseButton`
  (params (Key :type "Key Structure"))
  (:`Pressed`
    (set `self.isRotating` true))
  (:`Released`
    (set `self.isRotating` false)))

(event `InputAxisKey|MouseX`
  (params (AxisValue :type "Float (single-precision)"))
  (if (`self.isRotating`)
    (`SceneComponent.K2_AddLocalRotation` (`self.CameraRoot`) (`KismetMathLibrary.MakeRotator` 0.0 0.0 (* AxisValue 1.0)) false false)))

(event `InputAxisKey|MouseY`
  (params (AxisValue :type "Float (single-precision)"))
  (if (`self.isRotating`)
    (`SceneComponent.K2_AddLocalRotation` (`self.SpringArm`) (`KismetMathLibrary.MakeRotator` 0.0 (* AxisValue 1.0)) false false)))

(fn `UserConstructionScript`)