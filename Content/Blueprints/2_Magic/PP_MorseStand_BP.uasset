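; Puzzle stand that flashes a spotlight and beeps the Morse code for R'LYEH, then spawns an IP_ArchLeft item when solved.
; Interacting while unsolved changes the view and starts the signal, which repeats if the player is still in the Puzzle state after each pass.
; Dot and Dash play sounds and return their durations to the BeepGap macro, which times each flash.
; A red light precedes each pass.
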(event `self.ReceiveBeginPlay`
  (`SceneComponent.SetVisibility` (`self.SpotLight`) false false))

(event `self.OnInteract`
  (params (Player :type "PlayerCharacter Object Reference"))
  (if (not (`self.bIsSolved`))
    (bind _asbp_player_character (cast `/Game/Blueprints/BP_PlayerCharacter` Player))
    (`PlayerCharacter.OnMessageUpdate` _asbp_player_character "")
    (`self.ChangeView`)
    (`self.Start Signal` _asbp_player_character)))

(event `self.OnSolve`
  (`|SpawnActorFromClass` "/Game/Blueprints/2_Magic/IP_ArchLeft.IP_ArchLeft_C" (`SceneComponent.K2_GetComponentToWorld` (`self.Item Spawn`)) "AlwaysSpawn" "OverrideRootScale" null null))

(event `Reset Signal`
  (bind _spotlight (`self.SpotLight`))
  (`LightComponent.SetLightColor` _spotlight (struct :`R` 1.0 :`A` 1.0) true)
  (`SceneComponent.ToggleVisibility` _spotlight false))

(event `Start Signal`
  (params (Player :type "/Game/Blueprints/BP_PlayerCharacter Object Reference"))
  (bind _spotlight (`self.SpotLight`))
  (if (`|EnumEquality` (`PlayerCharacter.State` Player) "Puzzle") :!label _label
    (`self.Reset Signal`)
    (`KismetSystemLibrary.Delay` 2.0)
    (`LightComponent.SetLightColor` _spotlight (struct :`R` 1.0 :`G` 1.0 :`B` 1.0 :`A` 1.0) true)
    (`SceneComponent.ToggleVisibility` _spotlight false)
    (bind _duration (`self.Dot`))
    (`self.Beep Gap` _duration
      (:`End`
        (bind _duration_2 (`self.Dash`))
        (`self.Beep Gap` _duration_2
          (:`End`
            (bind _duration_3 (`self.Dot`))
            (`self.Beep Gap` _duration_3
              (:`End`
                (`KismetSystemLibrary.Delay` 0.7)
                (bind _duration_4 (`self.Dot`))
                (`self.Beep Gap` _duration_4
                  (:`End`
                    (bind _duration_5 (`self.Dash`))
                    (`self.Beep Gap` _duration_5
                      (:`End`
                        (bind _duration_6 (`self.Dash`))
                        (`self.Beep Gap` _duration_6
                          (:`End`
                            (bind _duration_7 (`self.Dash`))
                            (`self.Beep Gap` _duration_7
                              (:`End`
                                (bind _duration_8 (`self.Dash`))
                                (`self.Beep Gap` _duration_8
                                  (:`End`
                                    (bind _duration_9 (`self.Dot`))
                                    (`self.Beep Gap` _duration_9
                                      (:`End`
                                        (`KismetSystemLibrary.Delay` 0.7)
                                        (bind _duration_10 (`self.Dot`))
                                        (`self.Beep Gap` _duration_10
                                          (:`End`
                                            (bind _duration_11 (`self.Dash`))
                                            (`self.Beep Gap` _duration_11
                                              (:`End`
                                                (bind _duration_12 (`self.Dot`))
                                                (`self.Beep Gap` _duration_12
                                                  (:`End`
                                                    (bind _duration_13 (`self.Dot`))
                                                    (`self.Beep Gap` _duration_13
                                                      (:`End`
                                                        (`KismetSystemLibrary.Delay` 0.7)
                                                        (bind _duration_14 (`self.Dash`))
                                                        (`self.Beep Gap` _duration_14
                                                          (:`End`
                                                            (bind _duration_15 (`self.Dot`))
                                                            (`self.Beep Gap` _duration_15
                                                              (:`End`
                                                                (bind _duration_16 (`self.Dash`))
                                                                (`self.Beep Gap` _duration_16
                                                                  (:`End`
                                                                    (bind _duration_17 (`self.Dash`))
                                                                    (`self.Beep Gap` _duration_17
                                                                      (:`End`
                                                                        (`KismetSystemLibrary.Delay` 0.7)
                                                                        (bind _duration_18 (`self.Dot`))
                                                                        (`self.Beep Gap` _duration_18
                                                                          (:`End`
                                                                            (`KismetSystemLibrary.Delay` 0.7)
                                                                            (bind _duration_19 (`self.Dot`))
                                                                            (`self.Beep Gap` _duration_19
                                                                              (:`End`
                                                                                (bind _duration_20 (`self.Dot`))
                                                                                (`self.Beep Gap` _duration_20
                                                                                  (:`End`
                                                                                    (bind _duration_21 (`self.Dot`))
                                                                                    (`self.Beep Gap` _duration_21
                                                                                      (:`End`
                                                                                        (bind _duration_22 (`self.Dot`))
                                                                                        (`self.Beep Gap` _duration_22
                                                                                          (:`End`
                                                                                            (`KismetSystemLibrary.Delay` 0.7)
                                                                                            (goto _label)))))))))))))))))))))))))))))))))))))))))))))))

(event `R`)

(event `'`)

(event `L`)

(event `Y`)

(event `E`)

(event `H`)

(fn `Dash`
  (returns (Duration :type "Float (double-precision)"))
  (bind _dash_sound (`self.Dash Sound`))
  (`SceneComponent.ToggleVisibility` (`self.SpotLight`) false)
  (`GameplayStatics.PlaySoundAtLocation` _dash_sound (`SceneComponent.K2_GetComponentLocation` (`self.Speaker`)) (struct) 1.0 1.0 0.0 "/Game/Audio/BeepFallOff.BeepFalloff" null null)
  (return (`SoundBase.Duration` _dash_sound)))

(fn `Dot`
  (returns (Duration :type "Float (double-precision)"))
  (bind _dot_sound (`self.Dot Sound`))
  (`SceneComponent.ToggleVisibility` (`self.SpotLight`) false)
  (`GameplayStatics.PlaySoundAtLocation` _dot_sound (`SceneComponent.K2_GetComponentLocation` (`self.Speaker`)) (struct) 1.0 1.0 0.0 "/Game/Audio/BeepFallOff.BeepFalloff" null null)
  (return (`SoundBase.Duration` _dot_sound)))

(fn `UserConstructionScript`)