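; PieceSpawner is a clickable puzzle part that places a visual piece on a gate when solved.
; Clicking its mesh asks the linked Item to check the used item.
; Solve spawns a DummyItem slightly offset along world X, passes Item to CorrectMesh, then attaches it to the Gate, keeping its world transform.
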(event `self.PuzzlePartMeshComponent.OnClicked`
  (params (TouchedComponent :type "PrimitiveComponent Object Reference") (ButtonPressed :type "Key Structure"))
  (`ItemComponent.CheckUsedItem` (`self.Item`)))

(event `self.Solve`
  (bind (_returnvalue_location _returnvalue_rotation _returnvalue_scale) (`KismetMathLibrary.BreakTransform` (`self.GetTransform`)))
  (bind _returnvalue (`|SpawnActorFromClass` "/Game/Blueprints/DummyItem.DummyItem_C" (`KismetMathLibrary.MakeTransform` (+ _returnvalue_location (60.0 0.0 0.0)) _returnvalue_rotation _returnvalue_scale) "AlwaysSpawn" "OverrideRootScale" null null))
  (`/Game/Blueprints/DummyItem.Correct Mesh` _returnvalue (`self.Item`))
  (`self.K2_AttachToActor` _returnvalue (`self.Gate`) "None" "KeepWorld" "KeepWorld" "KeepWorld" true))

(fn `UserConstructionScript`)