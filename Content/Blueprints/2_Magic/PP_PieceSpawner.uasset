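; PP_PieceSpawner is a clickable puzzle part that places arch pieces on a Gate.
; Hovering its mesh shows a hand cursor, and clicking checks the used item.
; Solve switches on the item name to pick the left or right arch DummyItem child actor on the Gate.
; That actor gets its mesh corrected from the item and moves to the Gate's Handle location.
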(event `self.PuzzlePartMeshComponent.OnClicked`
  (params (TouchedComponent :type "PrimitiveComponent Object Reference") (ButtonPressed :type "Key Structure"))
  (`ItemComponent.CheckUsedItem` (`self.Item`))
  (set `PlayerController.CurrentMouseCursor` "Default" (`GameplayStatics.GetPlayerController` 0)))

(event `self.Solve`
  (bind _gate (`self.Gate`))
  (bind _returnvalue (`SceneComponent.K2_GetComponentLocation` (`Puzzle.Handle` _gate)))
  (bind _childactor (`ChildActorComponent.ChildActor` (`/Game/Blueprints/2_Magic/PZ_Gate.T5` _gate)))
  (bind _childactor_2 (`ChildActorComponent.ChildActor` (`/Game/Blueprints/2_Magic/PZ_Gate.T3` _gate)))
  (switch `string` (`KismetTextLibrary.Conv_TextToString` (`ItemComponent.ItemName` (`self.Item`)))
    (:`Arch's Left Part`
      (bind _asdummy_item (cast `/Game/Blueprints/DummyItem` _childactor))
      (`/Game/Blueprints/DummyItem.Correct Mesh` _asdummy_item (`self.Item`))
      (`self.K2_SetActorLocation` _childactor _returnvalue false false))
    (:`Arch's Right Part`
      (bind _asdummy_item_2 (cast `/Game/Blueprints/DummyItem` _childactor_2))
      (`/Game/Blueprints/DummyItem.Correct Mesh` _asdummy_item_2 (`self.Item`))
      (`self.K2_SetActorLocation` _childactor_2 _returnvalue false false))))

(event `self.PuzzlePartMeshComponent.OnEndCursorOver`
  (params (TouchedComponent :type "PrimitiveComponent Object Reference"))
  (set `PlayerController.CurrentMouseCursor` "Default" (`GameplayStatics.GetPlayerController` 0)))

(event `self.PuzzlePartMeshComponent.OnBeginCursorOver`
  (params (TouchedComponent :type "PrimitiveComponent Object Reference"))
  (set `PlayerController.CurrentMouseCursor` "Hand" (`GameplayStatics.GetPlayerController` 0)))

(fn `UserConstructionScript`)