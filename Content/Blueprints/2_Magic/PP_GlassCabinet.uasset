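; Puzzle-part Blueprint for a glass cabinet that opens when solved and reveals a cabinet key.
; Clicking its interact collision calls CheckUsedItem on Item to check the item being used.
; The Solve event spawns I_CabinetKey snapped to the Doors socket, instantly rotates the doors 90 degrees and disables the interact collision.
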(event `self.PuzzlePartInteractCollision.OnClicked`
  (params (TouchedComponent :type "PrimitiveComponent Object Reference") (ButtonPressed :type "Key Structure"))
  (`ItemComponent.CheckUsedItem` (`self.Item`)))

(event `self.Solve`
  (bind _returnvalue (`|SpawnActorFromClass` "/Game/Blueprints/2_Magic/I_CabinetKey.I_CabinetKey_C" (`self.GetTransform`) "AlwaysSpawn" "OverrideRootScale" null null))
  (`self.K2_AttachToComponent` _returnvalue (`self.Doors`) "Socket" "SnapToTarget" "SnapToTarget" "SnapToTarget" true)
  (`SceneComponent.K2_AddRelativeRotation` (`self.Doors`) (struct :`Yaw` 90.0) false false)
  (`PrimitiveComponent.SetCollisionEnabled` (`self.PuzzlePartInteractCollision`) "NoCollision"))

(fn `UserConstructionScript`)