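; Magic puzzle actor that solves once three of its linked Places are solved, raising its static mesh.
; On BeginPlay it binds to each Place's solve event, and every firing recounts solved Places with debug prints.
; A count of exactly three triggers OnSolve, which sets IsSolved.
; Interacting while unsolved shows the player a hint to place more stones, while interacting once solved re-runs OnSolve, lifting the mesh again.
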(event `self.ReceiveBeginPlay`
  (for _array_element (`self.Places`)
    (add `PuzzlePart.OnSolve` _array_element (delegate `Test`))))

(event `Test`
  (for _array_element (`self.Places`)
    (if (`PuzzlePart.bIsSolved` _array_element)
      (`/Engine/EditorBlueprintResources/StandardMacros.IncrementInt` (`self.Tes`)
        (:`  `
          (`KismetSystemLibrary.PrintString` (`KismetStringLibrary.Conv_IntToString` (`self.Tes`)))))))
  (if (== (`self.Tes`) 3)
    (`self.OnSolve`)
    (else
      (`KismetSystemLibrary.PrintString` "Not Enough")
      (set `self.Tes` 0))))

(event `self.OnInteract`
  (params (Player :type "PlayerCharacter Object Reference"))
  (if (`self.bIsSolved`)
    (`self.OnSolve`)
    (else
      (bind _asbp_player_character (cast `/Game/Blueprints/BP_PlayerCharacter` Player))
      (`PlayerCharacter.OnMessageUpdate` _asbp_player_character "Plce more weird Stones"))))

(event `self.OnSolve`
  (`SceneComponent.K2_AddRelativeLocation` (`self.StaticMesh`) (0.0 0.0 30.0) true false)
  (set `self.bIsSolved` true))

(fn `UserConstructionScript`)