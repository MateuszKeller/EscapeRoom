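; GateT is a mouse-driven drag puzzle that triggers its Answerer, apparently a gate, when solved.
; Clicking traces from the cursor to grab a Movable component, and Tick sweeps it along world Y/Z with the grab offset and fixed X.
; Overlapping Trigger_1 marks it solved; mouse release then runs a timeline turning PuzzleCamera toward the Answerer while calling Answer each update.
; Afterwards it hides the cursor, aims player control at the Answerer and calls ChangeView.
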(event `self.ReceiveTick`
  (params (DeltaSeconds :type "Float (single-precision)"))
  (bind _dragged_object (`self.Dragged Object`))
  (bind _dragged_object_2 (`self.Dragged Object`))
  (bind (_worldlocation _worlddirection) (`PlayerController.DeprojectMousePositionToWorld` (`GameplayStatics.GetPlayerController` 0)))
  (bind _returnvalue_x (`KismetMathLibrary.BreakVector` (`SceneComponent.K2_GetComponentLocation` _dragged_object_2)))
  (`/Engine/EditorBlueprintResources/StandardMacros.IsValid` _dragged_object
    (:`Is Valid`
      (`SceneComponent.K2_SetWorldLocation` _dragged_object_2 (`KismetMathLibrary.MakeVector` _returnvalue_x (.y (`KismetMathLibrary.InverseTransformLocation` (`KismetMathLibrary.Conv_VectorToTransform` (`self.Relative From Center`)) (+ _worldlocation (* _worlddirection (`KismetMathLibrary.Vector_Distance` _worldlocation (`SceneComponent.K2_GetComponentLocation` _dragged_object)))))) (.z (`KismetMathLibrary.InverseTransformLocation` (`KismetMathLibrary.Conv_VectorToTransform` (`self.Relative From Center`)) (+ _worldlocation (* _worlddirection (`KismetMathLibrary.Vector_Distance` _worldlocation (`SceneComponent.K2_GetComponentLocation` _dragged_object))))))) true false))))

(event `Key|LeftMouseButton`
  (params (Key :type "Key Structure"))
  (bind (_worldlocation _worlddirection) (`PlayerController.DeprojectMousePositionToWorld` (`GameplayStatics.GetPlayerController` 0)))
  (:`Pressed`
    (bind (_outhit _returnvalue) (`KismetSystemLibrary.LineTraceSingle` :`Start` _worldlocation :`End` (+ _worldlocation (* _worlddirection 200.0)) :`TraceChannel` "TraceTypeQuery1" :`bTraceComplex` true :`bIgnoreSelf` false))
    (if _returnvalue
      (if (`|EnumEquality` "Movable" (`SceneComponent.Mobility` (`.HitComponent` (`GameplayStatics.BreakHitResult` _outhit))))
        (set `self.Dragged Object` (`.HitComponent` (`GameplayStatics.BreakHitResult` _outhit)))
        (set `self.Relative From Center` (`KismetMathLibrary.InverseTransformLocation` (`KismetMathLibrary.Conv_VectorToTransform` (`SceneComponent.K2_GetComponentLocation` (`.HitComponent` (`GameplayStatics.BreakHitResult` _outhit)))) (`.Location` (`GameplayStatics.BreakHitResult` _outhit)))))))
  (:`Released`
    (set `self.Dragged Object` null)
    (if (`self.bIsSolved`)
      (`self.OnSolve`))))

(event `self.Trigger_4.OnComponentBeginOverlap`
  (params (OverlappedComponent :type "PrimitiveComponent Object Reference") (OtherActor :type "Actor Object Reference") (OtherComp :type "PrimitiveComponent Object Reference") (OtherBodyIndex :type Integer) (bFromSweep :type Boolean) (SweepResult :type "HitResult Structure (by ref)"))
  (`KismetSystemLibrary.PrintString` "Hit"))

(event `self.Trigger_4.OnComponentEndOverlap`
  (params (OverlappedComponent :type "PrimitiveComponent Object Reference") (OtherActor :type "Actor Object Reference") (OtherComp :type "PrimitiveComponent Object Reference") (OtherBodyIndex :type Integer))
  (`KismetSystemLibrary.PrintString` "Aut"))

(event `self.Trigger_1.OnComponentBeginOverlap`
  (params (OverlappedComponent :type "PrimitiveComponent Object Reference") (OtherActor :type "Actor Object Reference") (OtherComp :type "PrimitiveComponent Object Reference") (OtherBodyIndex :type Integer) (bFromSweep :type Boolean) (SweepResult :type "HitResult Structure (by ref)"))
  (set `self.bIsSolved` true))

(event `self.OnSolve`
  (bind _returnvalue (`GameplayStatics.GetPlayerController` 0))
  (bind _puzzlecamera (`self.PuzzleCamera`))
  (set `self.Gate Loc` (`SceneComponent.K2_GetComponentLocation` (`self.GetComponentByClass` (`self.Answerer`) "/Script/Engine.SceneComponent")))
  (set `self.Camera Loc` (`SceneComponent.K2_GetComponentLocation` _puzzlecamera))
  (set `self.Camera Rot` (`SceneComponent.K2_GetComponentRotation` _puzzlecamera))
  (bind (_direction _camera_to_gate) (`Timeline|Camera Movement`)
    (:`Update`
      (`SceneComponent.K2_SetWorldRotation` (`self.PuzzleCamera`) (`KismetMathLibrary.RLerp` (`self.Camera Rot`) (`KismetMathLibrary.FindLookAtRotation` (`self.Camera Loc`) (`self.Gate Loc`)) _camera_to_gate true) false false)
      (`PuzzleAnswerer.Answer` (`self.Answerer`)))
    (:`Finished`
      (set `PlayerController.bShowMouseCursor` false _returnvalue)
      (`Controller.SetControlRotation` _returnvalue (`KismetMathLibrary.FindLookAtRotation` (`SceneComponent.K2_GetComponentLocation` (`self.GetComponentByClass` (`GameplayStatics.GetPlayerCharacter` 0) "/Script/Engine.CameraComponent")) (`self.Gate Loc`)))
      (`KismetSystemLibrary.Delay` 0.5)
      (`self.ChangeView`))))

(fn `UserConstructionScript`)