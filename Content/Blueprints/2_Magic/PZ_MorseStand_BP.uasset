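; Morse code puzzle stand that switches view on interaction and loops "R'LYEH" as speaker beeps and spotlight flashes.
; Repeat steps through per-letter events via MultiGates and hand-tuned delays, with a red light marking each loop start.
; DotDash times each flash by sound duration and halts playback when the player leaves the Puzzle state.
; Solving switches view again and spawns the IP_ArchLeft item, moved vertically by a timeline.
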(event `self.ReceiveBeginPlay`
  (`self.Reset Light`))

(event `self.OnInteract`
  (params (Player :type "PlayerCharacter Object Reference"))
  (if (`self.bIsSolved`)
    _
    (elif (`self.bHasStoppedPlaying`)
      (bind _asbp_player_character (cast `/Game/Blueprints/BP_PlayerCharacter` Player))
      (if (`PlayerCharacter.bShowOutline` _asbp_player_character)
        (`Interactable.OnStopLooking`)
        (else
          (`PlayerCharacter.OnMessageUpdate` _asbp_player_character "")))
      (`self.ChangeView`)
      (`self.Start Signal`))))

(event `self.OnSolve`
  (`self.ChangeView`)
  (bind _returnvalue (`|SpawnActorFromClass` "/Game/Blueprints/2_Magic/IP_ArchLeft.IP_ArchLeft_C" (`SceneComponent.K2_GetComponentToWorld` (`self.Item Spawn`)) "AlwaysSpawn" "OverrideRootScale" null null))
  (bind (_direction _movement) (`Timeline|Item`)
    (:`Update`
      (if (`KismetSystemLibrary.IsValid` _returnvalue)
        (bind (_returnvalue_x _returnvalue_y) (`KismetMathLibrary.BreakVector` (`self.K2_GetActorLocation` _returnvalue)))
        (`self.K2_SetActorLocation` _returnvalue (`KismetMathLibrary.MakeVector` _returnvalue_x _returnvalue_y (+ _movement 0.0)) false false)))))

(event `R`
  (if (`self.Does Play Morse`)
    (`|MultiGate` false :!label _label
      (:`Out 0`
        (bind _duration (`self.Dot Dash` (`self.Dot Sound`)))
        (`self.Beep Gap` _duration
          (:`End`
            _)))
      (:`Out 1`
        (bind _duration_2 (`self.Dot Dash` (`self.Dash Sound`)))
        (`self.Beep Gap` _duration_2
          (:`End`
            _)))
      (:`Out 2`
        (bind _duration_3 (`self.Dot Dash` (`self.Dot Sound`)))
        (`self.Beep Gap` _duration_3
          (:`End`
            (`KismetSystemLibrary.Delay` 0.7)
            (goto _label :!via `Reset`)))))
    (`self.R`)
    (else
      (goto _label :!via `Reset`))))

(event `Start Signal`
  (set `self.Does Play Morse` true)
  (set `self.bHasStoppedPlaying` false)
  (`self.Repeat`))

(event `Repeat`
  (if (`self.Does Play Morse`)
    (`|MultiGate` false true :!label _label_2
      (:`Out 0`
        (`self.End Start`)
        (`KismetSystemLibrary.Delay` 1.5))
      (:`Out 1`
        (`self.R`)
        (`KismetSystemLibrary.Delay` 2.95))
      (:`Out 2`
        (`self.'`)
        (`KismetSystemLibrary.Delay` 6.16))
      (:`Out 3`
        (`self.l`)
        (`KismetSystemLibrary.Delay` 3.54))
      (:`Out 4`
        (`self.y`)
        (`KismetSystemLibrary.Delay` 4.5))
      (:`Out 5`
        (`self.e`)
        (`KismetSystemLibrary.Delay` 1.29))
      (:`Out 6`
        (`self.h`)
        (`KismetSystemLibrary.Delay` 3.06)))
    (`self.Repeat`)
    (else
      (`self.Reset Light`)
      (goto _label_2 :!via `Reset`))))

(event `'`
  (bind _dash_sound (`self.Dash Sound`))
  (if (`self.Does Play Morse`)
    (`|MultiGate` false :!label _label_3
      (:`Out 0`
        (bind _duration (`self.Dot Dash` (`self.Dot Sound`)))
        (`self.Beep Gap` _duration
          (:`End`
            _)))
      (:`Out 1`
        (bind _duration_2 (`self.Dot Dash` _dash_sound))
        (`self.Beep Gap` _duration_2
          (:`End`
            _)))
      (:`Out 2`
        (bind _duration_3 (`self.Dot Dash` _dash_sound))
        (`self.Beep Gap` _duration_3
          (:`End`
            _)))
      (:`Out 3`
        (bind _duration_4 (`self.Dot Dash` _dash_sound))
        (`self.Beep Gap` _duration_4
          (:`End`
            _)))
      (:`Out 4`
        (bind _duration_5 (`self.Dot Dash` _dash_sound))
        (`self.Beep Gap` _duration_5
          (:`End`
            _)))
      (:`Out 5`
        (bind _duration_6 (`self.Dot Dash` (`self.Dot Sound`)))
        (`self.Beep Gap` _duration_6
          (:`End`
            (`KismetSystemLibrary.Delay` 0.7)
            (goto _label_3 :!via `Reset`)))))
    (`self.'`)
    (else
      (goto _label_3 :!via `Reset`))))

(event `End Start`
  (bind _spotlight (`self.SpotLight`))
  (`LightComponent.SetLightColor` _spotlight (struct :`R` 1.0 :`A` 1.0) true)
  (`SceneComponent.SetVisibility` _spotlight true false)
  (`KismetSystemLibrary.Delay` 1.5)
  (`LightComponent.SetLightColor` _spotlight (struct :`R` 1.0 :`G` 1.0 :`B` 1.0 :`A` 1.0) true)
  (`SceneComponent.SetVisibility` _spotlight false false))

(event `Reset Light`
  (bind _spotlight (`self.SpotLight`))
  (`LightComponent.SetLightColor` _spotlight (struct :`R` 1.0 :`A` 1.0) true)
  (`SceneComponent.SetVisibility` _spotlight false false)
  (set `self.bHasStoppedPlaying` true))

(event `L`
  (bind _dot_sound (`self.Dot Sound`))
  (if (`self.Does Play Morse`)
    (`|MultiGate` false :!label _label_4
      (:`Out 0`
        (bind _duration (`self.Dot Dash` (`self.Dot Sound`)))
        (`self.Beep Gap` _duration
          (:`End`
            _)))
      (:`Out 1`
        (bind _duration_2 (`self.Dot Dash` (`self.Dash Sound`)))
        (`self.Beep Gap` _duration_2
          (:`End`
            _)))
      (:`Out 2`
        (bind _duration_3 (`self.Dot Dash` _dot_sound))
        (`self.Beep Gap` _duration_3
          (:`End`
            _)))
      (:`Out 3`
        (bind _duration_4 (`self.Dot Dash` _dot_sound))
        (`self.Beep Gap` _duration_4
          (:`End`
            (`KismetSystemLibrary.Delay` 0.7)
            (goto _label_4 :!via `Reset`)))))
    (`self.L`)
    (else
      (goto _label_4 :!via `Reset`))))

(event `Y`
  (bind _dash_sound (`self.Dash Sound`))
  (if (`self.Does Play Morse`)
    (`|MultiGate` false :!label _label_5
      (:`Out 0`
        (bind _duration (`self.Dot Dash` (`self.Dash Sound`)))
        (`self.Beep Gap` _duration
          (:`End`
            _)))
      (:`Out 1`
        (bind _duration_2 (`self.Dot Dash` (`self.Dot Sound`)))
        (`self.Beep Gap` _duration_2
          (:`End`
            _)))
      (:`Out 2`
        (bind _duration_3 (`self.Dot Dash` _dash_sound))
        (`self.Beep Gap` _duration_3
          (:`End`
            _)))
      (:`Out 3`
        (bind _duration_4 (`self.Dot Dash` _dash_sound))
        (`self.Beep Gap` _duration_4
          (:`End`
            (`KismetSystemLibrary.Delay` 0.7)
            (goto _label_5 :!via `Reset`)))))
    (`self.Y`)
    (else
      (goto _label_5 :!via `Reset`))))

(event `E`
  (if (`self.Does Play Morse`)
    (bind _duration (`self.Dot Dash` (`self.Dot Sound`)))
    (`self.Beep Gap` _duration
      (:`End`
        (`KismetSystemLibrary.Delay` 0.7)))))

(event `H`
  (bind _dot_sound (`self.Dot Sound`))
  (if (`self.Does Play Morse`)
    (`|MultiGate` false :!label _label_6
      (:`Out 0`
        (bind _duration (`self.Dot Dash` _dot_sound))
        (`self.Beep Gap` _duration
          (:`End`
            _)))
      (:`Out 1`
        (bind _duration_2 (`self.Dot Dash` _dot_sound))
        (`self.Beep Gap` _duration_2
          (:`End`
            _)))
      (:`Out 2`
        (bind _duration_3 (`self.Dot Dash` _dot_sound))
        (`self.Beep Gap` _duration_3
          (:`End`
            _)))
      (:`Out 3`
        (bind _duration_4 (`self.Dot Dash` _dot_sound))
        (`self.Beep Gap` _duration_4
          (:`End`
            (`KismetSystemLibrary.Delay` 0.7)
            (goto _label_6 :!via `Reset`)))))
    (`self.H`)
    (else
      (goto _label_6 :!via `Reset`))))

(fn `Check if still plating`
  (returns (`Does Play Morse` :type Boolean))
  (bind _is_correct (`/Game/Libraries/HUDFormatingLibrary.ComparePlayerState` "Puzzle"))
  (if (not _is_correct)
    (set `self.Does Play Morse` false))
  (return (`self.Does Play Morse`)))

(fn `Dot Dash`
  (params (Sound :type "SoundBase Object Reference"))
  (returns (Duration :type "Float (double-precision)"))
  (bind _does_play_morse (`self.Check if still plating`))
  (if _does_play_morse
    (`|ExecutionSequence`
      (:`then_0`
        (`SceneComponent.SetVisibility` (`self.SpotLight`) true false))
      (:`then_1`
        (`GameplayStatics.PlaySoundAtLocation` Sound (`SceneComponent.K2_GetComponentLocation` (`self.Speaker`)) (struct) 1.0 1.0 0.0 "/Game/Audio/BeepFallOff.BeepFalloff" null null)
        (return (`SoundBase.Duration` Sound))))
    (else
      (return (`SoundBase.Duration` Sound)))))

(fn `UserConstructionScript`)