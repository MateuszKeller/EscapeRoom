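; BP_Item is an item actor that prompts the player to pick it up and can be rotated with the mouse.
; Look-at events set or clear the "Press E" message on the BP_PlayerCharacter's HUD.
; While the left mouse button is held, mouse axes add yaw and pitch to the actor's rotation.
; The Interact input calls Drop, whose logic, like pickup itself, is not defined in these graphs.
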(event `self.OnLookAt`
  (params (Player :type "PlayerCharacter Object Reference"))
  (bind _asbp_player_character (cast `/Game/Blueprints/BP_PlayerCharacter` Player))
  (`/Game/UI/HUD.UpdateMessage` (`/Game/Blueprints/BP_PlayerCharacter.HUD` _asbp_player_character) "Press E to pick up item"))

(event `self.StopLookAt`
  (params (Player :type "PlayerCharacter Object Reference"))
  (bind _asbp_player_character (cast `/Game/Blueprints/BP_PlayerCharacter` Player))
  (`/Game/UI/HUD.UpdateMessage` (`/Game/Blueprints/BP_PlayerCharacter.HUD` _asbp_player_character) ""))

(event `Key|LeftMouseButton`
  (params (Key :type "Key Structure"))
  (:`Pressed`
    (set `self.isRotating` true))
  (:`Released`
    (set `self.isRotating` false)))

(event `InputAxisKey|MouseX`
  (params (AxisValue :type "Float (single-precision)"))
  (if (`self.isRotating`)
    (`self.K2_SetActorRotation` (`KismetMathLibrary.ComposeRotators` (`self.K2_GetActorRotation`) (`KismetMathLibrary.MakeRotator` 0.0 0.0 (* -5 AxisValue))))))

(event `InputAxisKey|MouseY`
  (params (AxisValue :type "Float (single-precision)"))
  (if (`self.isRotating`)
    (`self.K2_SetActorRotation` (`KismetMathLibrary.ComposeRotators` (`self.K2_GetActorRotation`) (`KismetMathLibrary.MakeRotator` 0.0 (* -5 AxisValue))))))

(event `InputAction|Interact`
  (params (Key :type "Key Structure"))
  (:`Pressed`
    (`self.Drop`)))

(fn `UserConstructionScript`)