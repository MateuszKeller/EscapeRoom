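; A test answerer actor with a clickable door that reacts to the item the player is using.
; Clicking the door runs the item's used-item check: success paints both material slots rainbow and removes the item through the cached player character, while failure shows the player a Polish wrong-item message.
; A separate Answer event opens the door by snapping its relative rotation, independent of the click logic.
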(event `self.ReceiveBeginPlay`
  (bind _asbp_player_character (cast `/Game/Blueprints/BP_PlayerCharacter` (`GameplayStatics.GetPlayerCharacter` 0)))
  (set `self.Player` _asbp_player_character))

(event `self.Door.OnClicked`
  (params (TouchedComponent :type "PrimitiveComponent Object Reference") (ButtonPressed :type "Key Structure"))
  (bind _returnvalue (`ItemComponent.CheckUsedItem` (`self.Item`)))
  (if _returnvalue
    (`PrimitiveComponent.SetMaterial` (`self.Door`) 0 "/Game/Materials/M_Rainbow.M_Rainbow")
    (`PrimitiveComponent.SetMaterial` (`self.Door`) 1 "/Game/Materials/M_Rainbow.M_Rainbow")
    (`PlayerCharacter.RemoveUsedItem` (`self.Player`))
    (else
      (`/Game/Blueprints/BP_PlayerCharacter.Display Message` (`self.Player`) "Inny przedmiot chopej"))))

(event `self.Answer`
  (`self.OpenTheDoor`))

(fn `OpenTheDoor`
  (`SceneComponent.K2_SetRelativeRotation` (`self.Door`) (struct :`Yaw` 90.0) false false))

(fn `UserConstructionScript`)