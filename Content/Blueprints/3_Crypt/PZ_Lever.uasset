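; Crypt puzzle actor in which the player mouse-drags a lever along a spline, with three clickable pieces controlling stops.
; A mouse trace picks up a movable component; Tick projects the cursor, offset by the grab point, to the nearest spline point and moves the lever there with sweep.
; Each click rotates W1–W3 one step, disabling its stop's collision only at the target angle.
; Releasing the mouse calls OnSolve if IsSolved is set.
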(event `self.ReceiveTick`
  (params (DeltaSeconds :type "Float (single-precision)"))
  (bind _dragged_object (`self.Dragged Object`))
  (bind (_worldlocation _worlddirection) (`PlayerController.DeprojectMousePositionToWorld` (`GameplayStatics.GetPlayerController` 0)))
  (if (== _dragged_object (`Actor.RootComponent` (`ChildActorComponent.ChildActor` (`self.Lever`))))
    (`SceneComponent.K2_SetWorldLocation` (`self.Dragged Object`) (`SplineComponent.FindLocationClosestToWorldLocation` (`self.Spline`) (`KismetMathLibrary.InverseTransformLocation` (`KismetMathLibrary.Conv_VectorToTransform` (`self.Relative From Center`)) (+ _worldlocation (* _worlddirection (`KismetMathLibrary.Vector_Distance` _worldlocation (`SceneComponent.K2_GetComponentLocation` _dragged_object))))) "World") true false)
    (`SceneComponent.K2_SetWorldLocation` (`self.Lever`) (`SplineComponent.FindLocationClosestToWorldLocation` (`self.Spline`) (`KismetMathLibrary.InverseTransformLocation` (`KismetMathLibrary.Conv_VectorToTransform` (`self.Relative From Center`)) (+ _worldlocation (* _worlddirection (`KismetMathLibrary.Vector_Distance` _worldlocation (`SceneComponent.K2_GetComponentLocation` _dragged_object))))) "World") true false)))

(event `Key|LeftMouseButton`
  (params (Key :type "Key Structure"))
  (bind (_worldlocation _worlddirection) (`PlayerController.DeprojectMousePositionToWorld` (`GameplayStatics.GetPlayerController` 0)))
  (:`Pressed`
    (bind (_outhit _returnvalue) (`KismetSystemLibrary.LineTraceSingle` :`Start` _worldlocation :`End` (+ _worldlocation (* _worlddirection 200.0)) :`TraceChannel` "TraceTypeQuery1" :`bTraceComplex` true :`bIgnoreSelf` false))
    (if _returnvalue
      (if (`|EnumEquality` "Movable" (`SceneComponent.Mobility` (`.HitComponent` (`GameplayStatics.BreakHitResult` _outhit))))
        (set `self.Dragged Object` (`.HitComponent` (`GameplayStatics.BreakHitResult` _outhit)))
        (set `self.Relative From Center` (`KismetMathLibrary.InverseTransformLocation` (`KismetMathLibrary.Conv_VectorToTransform` (`SceneComponent.K2_GetComponentLocation` (`.HitComponent` (`GameplayStatics.BreakHitResult` _outhit)))) (`.Location` (`GameplayStatics.BreakHitResult` _outhit)))))))
  (:`Released`
    (set `self.Dragged Object` null)
    (if (`self.bIsSolved`)
      (`self.OnSolve`))))

(event `self.W1.OnClicked`
  (params (TouchedComponent :type "PrimitiveComponent Object Reference") (ButtonPressed :type "Key Structure"))
  (bind _stop1 (`self.Stop1`))
  (bind (_relativerotation_roll _relativerotation_pitch) (`KismetMathLibrary.BreakRotator` (`SceneComponent.RelativeRotation` (`self.W1`))))
  (`SceneComponent.K2_AddLocalRotation` TouchedComponent (struct :`Yaw` -30.0) true false)
  (if (`KismetMathLibrary.NearlyEqual_FloatFloat` _relativerotation_pitch -90.0 0.1)
    (`PrimitiveComponent.SetCollisionEnabled` _stop1 "NoCollision")
    (else
      (`PrimitiveComponent.SetCollisionEnabled` _stop1 "QueryAndPhysics"))))

(event `self.W2.OnClicked`
  (params (TouchedComponent :type "PrimitiveComponent Object Reference") (ButtonPressed :type "Key Structure"))
  (bind _stop2 (`self.Stop2`))
  (bind (_relativerotation_roll _relativerotation_pitch) (`KismetMathLibrary.BreakRotator` (`SceneComponent.RelativeRotation` (`self.W2`))))
  (`SceneComponent.K2_AddLocalRotation` TouchedComponent (struct :`Yaw` -30.0) false false)
  (if (`KismetMathLibrary.NearlyEqual_FloatFloat` _relativerotation_pitch -90.0 0.1)
    (`PrimitiveComponent.SetCollisionEnabled` _stop2 "NoCollision")
    (else
      (`PrimitiveComponent.SetCollisionEnabled` _stop2 "QueryAndPhysics"))))

(event `self.W3.OnClicked`
  (params (TouchedComponent :type "PrimitiveComponent Object Reference") (ButtonPressed :type "Key Structure"))
  (bind _stop3 (`self.Stop3`))
  (bind (_relativerotation_roll _relativerotation_pitch) (`KismetMathLibrary.BreakRotator` (`SceneComponent.RelativeRotation` (`self.W3`))))
  (`SceneComponent.K2_AddLocalRotation` TouchedComponent (struct :`Yaw` -30.0) false false)
  (if (`KismetMathLibrary.NearlyEqual_FloatFloat` _relativerotation_pitch -90.0 0.1)
    (`PrimitiveComponent.SetCollisionEnabled` _stop3 "NoCollision")
    (else
      (`PrimitiveComponent.SetCollisionEnabled` _stop3 "QueryAndPhysics"))))

(fn `UserConstructionScript`)