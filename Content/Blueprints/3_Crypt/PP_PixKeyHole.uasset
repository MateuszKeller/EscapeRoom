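; Clickable keyhole puzzle part for the Crypt level that reacts to item use and disappears once solved.
; Hovering its mesh switches the player's mouse cursor to a hand, and leaving or clicking restores the default.
; A click asks the Item to check the used item.
; A separate Solve event marks the part as solved and destroys the actor.
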(event `self.PuzzlePartMeshComponent.OnClicked`
  (params (TouchedComponent :type "PrimitiveComponent Object Reference") (ButtonPressed :type "Key Structure"))
  (set `PlayerController.CurrentMouseCursor` "Default" (`GameplayStatics.GetPlayerController` 0))
  (`ItemComponent.CheckUsedItem` (`self.Item`)))

(event `self.PuzzlePartMeshComponent.OnBeginCursorOver`
  (params (TouchedComponent :type "PrimitiveComponent Object Reference"))
  (set `PlayerController.CurrentMouseCursor` "Hand" (`GameplayStatics.GetPlayerController` 0)))

(event `self.PuzzlePartMeshComponent.OnEndCursorOver`
  (params (TouchedComponent :type "PrimitiveComponent Object Reference"))
  (set `PlayerController.CurrentMouseCursor` "Default" (`GameplayStatics.GetPlayerController` 0)))

(event `self.Solve`
  (set `self.bIsSolved` true)
  (`self.K2_DestroyActor`))

(fn `UserConstructionScript`)