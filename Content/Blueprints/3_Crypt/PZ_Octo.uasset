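; PZ_Octo is a crypt puzzle where the player mouse-drags pieces along splines and clicks a rotator to turn it in steps.
; A trace from the cursor picks a Movable component, and Tick snaps it to the closest point on its parent spline, offset by the grab point.
; On release, four pieces near zero relative X mark it solved, spawning an actor at the Handle and changing view.
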(event `self.ReceiveBeginPlay`)

(event `self.ReceiveTick`
  (params (DeltaSeconds :type "Float (single-precision)"))
  (bind _dragged_object (`self.Dragged Object`))
  (bind (_worldlocation _worlddirection) (`PlayerController.DeprojectMousePositionToWorld` (`GameplayStatics.GetPlayerController` 0)))
  (`/Engine/EditorBlueprintResources/StandardMacros.IsValid` _dragged_object
    (:`Is Valid`
      (bind _asspline_component (cast `SplineComponent` (`SceneComponent.GetAttachParent` _dragged_object)))
      (`SceneComponent.K2_SetWorldLocation` (`self.Dragged Object`) (`SplineComponent.FindLocationClosestToWorldLocation` _asspline_component (`KismetMathLibrary.InverseTransformLocation` (`KismetMathLibrary.Conv_VectorToTransform` (`self.Relative From Center`)) (+ _worldlocation (* _worlddirection (`KismetMathLibrary.Vector_Distance` _worldlocation (`SceneComponent.K2_GetComponentLocation` _dragged_object))))) "World") true false))))

(event `Key|LeftMouseButton`
  (params (Key :type "Key Structure"))
  (bind (_worldlocation _worlddirection) (`PlayerController.DeprojectMousePositionToWorld` (`GameplayStatics.GetPlayerController` 0)))
  (:`Pressed`
    (bind (_outhit _returnvalue) (`KismetSystemLibrary.LineTraceSingle` :`Start` _worldlocation :`End` (+ _worldlocation (* _worlddirection 200.0)) :`TraceChannel` "TraceTypeQuery1" :`bTraceComplex` true :`bIgnoreSelf` false))
    (if _returnvalue
      (if (`|EnumEquality` "Movable" (`SceneComponent.Mobility` (`.HitComponent` (`GameplayStatics.BreakHitResult` _outhit))))
        (set `self.Dragged Object` (`.HitComponent` (`GameplayStatics.BreakHitResult` _outhit)))
        (set `self.Relative From Center` (`KismetMathLibrary.InverseTransformLocation` (`KismetMathLibrary.Conv_VectorToTransform` (`SceneComponent.K2_GetComponentLocation` (`.HitComponent` (`GameplayStatics.BreakHitResult` _outhit)))) (`.Location` (`GameplayStatics.BreakHitResult` _outhit)))))))
  (:`Released`
    (`self.NewFunction_0`)
    (set `self.Dragged Object` null)
    (if (`self.bIsSolved`)
      (`self.OnSolve`))))

(event `self.Rotator.OnClicked`
  (params (TouchedComponent :type "PrimitiveComponent Object Reference") (ButtonPressed :type "Key Structure"))
  (`SceneComponent.K2_AddLocalRotation` TouchedComponent (struct :`Yaw` -30.0) false false))

(event `self.OnSolve`
  (bind (_returnvalue_location _returnvalue_rotation _returnvalue_scale) (`KismetMathLibrary.BreakTransform` (`SceneComponent.K2_GetComponentToWorld` (`self.Handle`))))
  (`|SpawnActorFromClass` "/Game/Blueprints/3_Crypt/I_GoldCrystal.I_GoldCrystal_C" (`KismetMathLibrary.MakeTransform` (+ (-5.0 0.0 0.0) _returnvalue_location) _returnvalue_rotation _returnvalue_scale) "AlwaysSpawn" "OverrideRootScale" null null)
  (`self.ChangeView`))

(fn `NewFunction_0`
  (bind _relativelocation_x (`KismetMathLibrary.BreakVector` (`SceneComponent.RelativeLocation` (`self.PW`))))
  (bind _relativelocation_x_2 (`KismetMathLibrary.BreakVector` (`SceneComponent.RelativeLocation` (`self.PN`))))
  (bind _relativelocation_x_3 (`KismetMathLibrary.BreakVector` (`SceneComponent.RelativeLocation` (`self.PE`))))
  (bind _relativelocation_x_4 (`KismetMathLibrary.BreakVector` (`SceneComponent.RelativeLocation` (`self.PS`))))
  (if (`KismetMathLibrary.NearlyEqual_FloatFloat` _relativelocation_x_2 0.0 0.1)
    (if (`KismetMathLibrary.NearlyEqual_FloatFloat` _relativelocation_x_3 0.0 0.1)
      (if (`KismetMathLibrary.NearlyEqual_FloatFloat` _relativelocation_x_4 0.0 0.1)
        (if (`KismetMathLibrary.NearlyEqual_FloatFloat` _relativelocation_x 0.0 0.1)
          (set `self.bIsSolved` true))))))

(fn `UserConstructionScript`)