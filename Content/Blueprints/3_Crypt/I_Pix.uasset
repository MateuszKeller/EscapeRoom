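; Crypt puzzle actor: a locked object with four spline sliders whose Top component is destroyed when the puzzle is solved.
; Destroying the KeyHole child actor shifts the four splines outward to expose the sliders.
; Left click line-traces from the cursor to grab a slider, which Tick drags to the closest point on its parent spline.
; On release, each slider is checked against its spline's mapped trigger, and all four inside opens it.
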(event `self.ReceiveBeginPlay`
  (add `Actor.OnDestroyed` (`ChildActorComponent.ChildActor` (`self.Key Hole`)) (delegate `Show Sliders`))
  (`self.Set Spline to Triggers`))

(event `Show Sliders`
  (params (DestroyedActor :type "Actor Object Reference"))
  (`self.Move Sliders`))

(event `self.ReceiveTick`
  (params (DeltaSeconds :type "Float (single-precision)"))
  (`self.Drag Along Spline`))

(event `Key|LeftMouseButton`
  (params (Key :type "Key Structure"))
  (bind (_worldlocation _worlddirection) (`PlayerController.DeprojectMousePositionToWorld` (`GameplayStatics.GetPlayerController` 0)))
  (:`Pressed`
    (if (not (`self.Open`))
      (`/Engine/EditorBlueprintResources/StandardMacros.IsValid` (`self.Dragged Object`)
        (:`Is Not Valid`
          (`WidgetBlueprintLibrary.SetInputMode_GameAndUIEx` (`GameplayStatics.GetPlayerController` 0) null "LockInFullscreen" false)
          (bind (_outhit _returnvalue) (`KismetSystemLibrary.LineTraceSingle` :`Start` _worldlocation :`End` (+ _worldlocation (* _worlddirection 200.0)) :`TraceChannel` "TraceTypeQuery1" :`bTraceComplex` true :`bIgnoreSelf` false))
          (if _returnvalue
            (bind _asspline_component (cast `SplineComponent` (`SceneComponent.GetAttachParent` (`.HitComponent` (`GameplayStatics.BreakHitResult` _outhit)))))
            (set `self.Coresponding Spline` _asspline_component)
            (set `self.Dragged Object` (`.HitComponent` (`GameplayStatics.BreakHitResult` _outhit)))
            (set `self.Relative From Center` (`KismetMathLibrary.InverseTransformLocation` (`KismetMathLibrary.Conv_VectorToTransform` (`SceneComponent.K2_GetComponentLocation` (`.HitComponent` (`GameplayStatics.BreakHitResult` _outhit)))) (`.Location` (`GameplayStatics.BreakHitResult` _outhit)))))))))
  (:`Released`
    (`self.Reset Click`)))

(fn `Drag Along Spline`
  (bind _dragged_object (`self.Dragged Object`))
  (bind (_worldlocation _worlddirection) (`PlayerController.DeprojectMousePositionToWorld` (`GameplayStatics.GetPlayerController` 0)))
  (`/Engine/EditorBlueprintResources/StandardMacros.IsValid` _dragged_object
    (:`Is Valid`
      (`SceneComponent.K2_SetWorldLocation` (`self.Dragged Object`) (`SplineComponent.FindLocationClosestToWorldLocation` (`self.Coresponding Spline`) (`KismetMathLibrary.InverseTransformLocation` (`KismetMathLibrary.Conv_VectorToTransform` (`self.Relative From Center`)) (+ _worldlocation (* _worlddirection (`KismetMathLibrary.Vector_Distance` _worldlocation (`SceneComponent.K2_GetComponentLocation` _dragged_object))))) "World") true false))))

(fn `Move Sliders`
  (`SceneComponent.K2_SetRelativeLocation` (`self.Spline_1`) (18.1 0.0 0.0) false false)
  (`SceneComponent.K2_SetRelativeLocation` (`self.Spline_2`) (0.0 18.1 0.0) false false)
  (`SceneComponent.K2_SetRelativeLocation` (`self.Spline_3`) (-18.1 0.0 0.0) false false)
  (`SceneComponent.K2_SetRelativeLocation` (`self.Spline_4`) (0.0 -18.1 0.0) false false))

(fn `Reset Click`
  (set `self.Open` true)
  (`WidgetBlueprintLibrary.SetInputMode_GameAndUIEx` (`GameplayStatics.GetPlayerController` 0) null "LockInFullscreen")
  (set `self.Dragged Object` null)
  (set `self.Coresponding Spline` null)
  (bind _keys (`BlueprintMapLibrary.Map_Keys` (`self.Splines to Triggers`)))
  (for _array_element _keys
    (bind _asprimitive_component (cast `PrimitiveComponent` (`SceneComponent.GetChildComponent` _array_element 0)))
    (bind _is_whole_inside (`/Game/Libraries/ActorLibrary.Is Whole Component Inside Volume` _asprimitive_component (`BlueprintMapLibrary.Map_Find` (`self.Splines to Triggers`) _array_element)))
    (if (not _is_whole_inside)
      (set `self.Open` false)
      (break)))
  (if (and (`self.Open`) (`KismetSystemLibrary.IsValid` (`self.Top`)))
    (`ActorComponent.K2_DestroyComponent` (`self.Top`))))

(fn `Set Spline to Triggers`
  (bind _splines_to_triggers (`self.Splines to Triggers`))
  (`BlueprintMapLibrary.Map_Add` _splines_to_triggers (`self.Spline_1`) (`self.Trigger_1`))
  (`BlueprintMapLibrary.Map_Add` _splines_to_triggers (`self.Spline_2`) (`self.Trigger_2`))
  (`BlueprintMapLibrary.Map_Add` _splines_to_triggers (`self.Spline_3`) (`self.Trigger_3`))
  (`BlueprintMapLibrary.Map_Add` _splines_to_triggers (`self.Spline_4`) (`self.Trigger_4`)))

(fn `UserConstructionScript`)