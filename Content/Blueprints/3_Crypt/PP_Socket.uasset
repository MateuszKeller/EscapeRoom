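; Crypt puzzle socket that takes a crystal item and shows it in place once solved.
; Hovering the puzzle mesh shows a hand cursor, and clicking an unsolved socket has its Item check the used item.
; Solve records the crystal's class, attaches a spawned DummyItem with the matching mesh at a rotated angle, and calls CallOnSolve.
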(event `self.PuzzlePartMeshComponent.OnClicked`
  (params (TouchedComponent :type "PrimitiveComponent Object Reference") (ButtonPressed :type "Key Structure"))
  (set `PlayerController.CurrentMouseCursor` "Default" (`GameplayStatics.GetPlayerController` 0))
  (if (not (`self.bIsSolved`))
    (`ItemComponent.CheckUsedItem` (`self.Item`))))

(event `self.Solve`
  (set `self.Used Crystal` (`ItemComponent.ItemClass` (`self.Item`)))
  (set `self.bIsSolved` true)
  (bind _returnvalue (`|SpawnActorFromClass` "/Game/Blueprints/DummyItem.DummyItem_C" (`self.GetTransform`) "AlwaysSpawn" "OverrideRootScale" null null))
  (`/Game/Blueprints/DummyItem.Correct Mesh` _returnvalue (`self.Item`))
  (`self.K2_AttachToActor` _returnvalue self "None" "SnapToTarget" "KeepRelative" "KeepRelative" true)
  (`self.K2_SetActorRelativeRotation` _returnvalue (struct :`Roll` 90.0) false false)
  (`self.OnSolve`))

(event `self.PuzzlePartMeshComponent.OnBeginCursorOver`
  (params (TouchedComponent :type "PrimitiveComponent Object Reference"))
  (set `PlayerController.CurrentMouseCursor` "Hand" (`GameplayStatics.GetPlayerController` 0)))

(event `self.PuzzlePartMeshComponent.OnEndCursorOver`
  (params (TouchedComponent :type "PrimitiveComponent Object Reference"))
  (set `PlayerController.CurrentMouseCursor` "Default" (`GameplayStatics.GetPlayerController` 0)))

(fn `UserConstructionScript`)