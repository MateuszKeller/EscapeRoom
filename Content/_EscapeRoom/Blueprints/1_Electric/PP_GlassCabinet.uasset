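; Clickable glass cabinet puzzle piece in the Electric escape room set that swings open when solved.
; Clicking its mesh has the Item member check the used item.
; The Solve event sets IsSolved and plays the Open timeline, which drives the mesh's relative roll while keeping pitch and yaw.
; BeginPlay attaches the mesh component with relative transform rules.
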(event `self.ReceiveBeginPlay`
  (`SceneComponent.K2_AttachToComponent` (`self.PPMeshComponent`) null "None" "KeepRelative" "KeepRelative" "KeepRelative" true))

(event `self.PPMeshComponent.OnClicked`
  (params (TouchedComponent :type "PrimitiveComponent Object Reference") (ButtonPressed :type "Key Structure"))
  (`ItemComponent.CheckUsedItem` (`self.Item`)))

(event `self.Solve`
  (bind _ppmeshcomponent (`self.PPMeshComponent`))
  (bind (_relativerotation_roll _relativerotation_pitch _relativerotation_yaw) (`KismetMathLibrary.BreakRotator` (`SceneComponent.RelativeRotation` _ppmeshcomponent)))
  (set `self.bIsSolved` true)
  (bind (_direction _open_angle) (`Timeline|Open`)
    (:`Update`
      (`SceneComponent.K2_SetRelativeRotation` _ppmeshcomponent (`KismetMathLibrary.MakeRotator` _open_angle _relativerotation_pitch _relativerotation_yaw) false false))))

(fn `UserConstructionScript`)