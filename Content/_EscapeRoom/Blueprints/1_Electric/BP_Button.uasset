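; BP_Button is a one-shot interactable push button in the escape room's Electric section that submits an answer to a linked Answerer.
; Looking at it shows an "[E] Press" prompt through the player's pointer text, as long as it is neither hidden nor pressed.
; Interacting clears the prompt, calls Answer on the Answerer, nudges the button inward with a swept relative move, and latches WasPressed to block further use.
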(event `self.OnInteract`
  (params (Player :type "PlayerCharacter Object Reference"))
  (if (`self.bHidden`)
    _
    (elif (not (`self.Was Pressed`))
      (`PlayerCharacter.OnPointerTextUpdate` Player "")
      (`PuzzleAnswerer.Answer` (`self.Answerer`))
      (`SceneComponent.K2_AddRelativeLocation` (`self.Button`) (-3.0 0.0 0.0) true false)
      (set `self.Was Pressed` true))))

(event `self.OnLookAt`
  (params (Player :type "PlayerCharacter Object Reference"))
  (if (`self.bHidden`)
    _
    (elif (not (`self.Was Pressed`))
      (`PlayerCharacter.OnPointerTextUpdate` Player "[E] Press"))))

(fn `UserConstructionScript`)