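; PP_Socket is a clickable crystal socket for a Crypt puzzle in the escape room.
; Clicking it while unsolved has its Item component check the item being used.
; Solve records the crystal class, broadcasts solved and crystal-used events, and applies the item's material to the socket mesh.
; It then spawns a DummyItem with the item's mesh and snaps it to the socket's Scene component.
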(event `self.PPMeshComponent.OnClicked`
  (params (TouchedComponent :type "PrimitiveComponent Object Reference") (ButtonPressed :type "Key Structure"))
  (set `PlayerController.CurrentMouseCursor` "Default" (`GameplayStatics.GetPlayerController` 0))
  (if (not (`self.bIsSolved`))
    (`ItemComponent.CheckUsedItem` (`self.Item`))))

(event `self.Solve`
  (bind _materialinterface (`ItemComponent.MaterialInterface` (`self.Item`)))
  (set `self.Used Crystal` (`ItemComponent.ItemClass` (`self.Item`)))
  (set `self.bIsSolved` true)
  (`self.OnSolve`)
  (`self.On Crystal Used` self _materialinterface)
  (`PrimitiveComponent.SetMaterial` (`self.PPMeshComponent`) 0 _materialinterface)
  (bind _returnvalue (`|SpawnActorFromClass` "/Game/_EscapeRoom/Blueprints/DummyItem.DummyItem_C" (`KismetMathLibrary.MakeTransform` (0.0 0.0 0.0)) "Undefined" "OverrideRootScale" null null))
  (`/Game/_EscapeRoom/Blueprints/DummyItem.Correct Mesh` _returnvalue (`self.Item`))
  (`self.K2_AttachToComponent` _returnvalue (`self.Scene`) "None" "SnapToTarget" "SnapToTarget" "KeepWorld" true))

(fn `UserConstructionScript`)