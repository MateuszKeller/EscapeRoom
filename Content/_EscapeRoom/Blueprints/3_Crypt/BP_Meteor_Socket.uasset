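; Crypt puzzle actor that recolours its three meteor parts when crystals are used in their linked sockets.
; The construction script gathers the Left, Middle and Right components into a Parts array.
; On BeginPlay it pairs each socket key in SocketsToParts with a part by index and binds to its OnCrystalUsed event.
; That event applies the supplied material to the matching part.
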(event `self.ReceiveBeginPlay`
  (bind _keys (`BlueprintMapLibrary.Map_Keys` (`self.Sockets to Parts`)))
  (for (_array_element _array_index) _keys
    (add `/Game/_EscapeRoom/Blueprints/3_Crypt/PP_Socket.On Crystal Used` _array_element (delegate `Recolour`))
    (`BlueprintMapLibrary.Map_Add` (`self.Sockets to Parts`) _array_element (`|GetArrayItem` (`self.Parts`) _array_index))))

(event `Recolour`
  (params (Socket :type "/Game/_EscapeRoom/Blueprints/3_Crypt/PP_Socket Object Reference") (Material :type "MaterialInterface Object Reference"))
  (`PrimitiveComponent.SetMaterial` (`BlueprintMapLibrary.Map_Find` (`self.Sockets to Parts`) Socket) 0 Material))

(fn `UserConstructionScript`
  (bind _parts (`self.Parts`))
  (`KismetArrayLibrary.Array_Add` _parts (`self.Left`))
  (`KismetArrayLibrary.Array_Add` _parts (`self.Middle`))
  (`KismetArrayLibrary.Array_Add` _parts (`self.Right`)))