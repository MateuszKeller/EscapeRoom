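; Player character Blueprint for an escape room game, linking the player to the game's HUD.
; On BeginPlay it starts a camera fade from black, caches the HUD from the escape room GameMode and broadcasts an empty keys update.
; DisplayMessage pushes text to that HUD and also prints it, and a QuitGame event exits the game.
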(event `self.ReceiveBeginPlay`
  (`PlayerCameraManager.StartCameraFade` :`self` (`GameplayStatics.GetPlayerCameraManager` 0) :`FromAlpha` 1.0 :`Duration` 2.0)
  (bind _asbp_gm_escape_room (cast `/Game/_EscapeRoom/Blueprints/BP_GM_Escape_Room` (`GameplayStatics.GetGameMode`)))
  (set `self.HUD` (`/Game/_EscapeRoom/Blueprints/BP_GM_Escape_Room.HUD` _asbp_gm_escape_room))
  (`self.OnKeysUpdate` ""))

(event `self.ReceiveTick`
  (params (DeltaSeconds :type "Float (single-precision)")))

(event `self.QuitGame`
  (`KismetSystemLibrary.QuitGame` null "Quit"))

(fn `Display Message`
  (params (Message :type Text))
  (`/Game/_EscapeRoom/UI/HUD.Update Text` (`self.HUD`) null Message)
  (`KismetSystemLibrary.PrintString` (`KismetTextLibrary.Conv_TextToString` Message)))

(fn `UserConstructionScript`)