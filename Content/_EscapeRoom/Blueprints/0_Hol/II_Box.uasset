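; II_Box is an inspectable escape-room box with a lid that opens on click.
; OnInteract clears the player's pointer text, starts inspection and fires the OnInspect dispatcher.
; Hovering over the lid switches the mouse cursor to a hand.
; Clicking resets the cursor and, while the box is closed, plays a timeline that rotates the lid on roll, setting IsOpen when finished.
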(event `self.OnInteract`
  (params (Player :type "PlayerCharacter Object Reference"))
  (`PlayerCharacter.OnPointerTextUpdate` Player "")
  (`self.Inspect` Player)
  (`self.OnInspect`))

(event `self.Lid.OnBeginCursorOver`
  (params (TouchedComponent :type "PrimitiveComponent Object Reference"))
  (set `PlayerController.CurrentMouseCursor` "Hand" (`GameplayStatics.GetPlayerController` 0)))

(event `self.Lid.OnEndCursorOver`
  (params (TouchedComponent :type "PrimitiveComponent Object Reference"))
  (set `PlayerController.CurrentMouseCursor` "Default" (`GameplayStatics.GetPlayerController` 0)))

(event `self.Lid.OnClicked`
  (params (TouchedComponent :type "PrimitiveComponent Object Reference") (ButtonPressed :type "Key Structure"))
  (set `PlayerController.CurrentMouseCursor` "Default" (`GameplayStatics.GetPlayerController` 0))
  (if (not (`self.IsOpen`))
    (bind (_direction _open_angle) (`Timeline|Lid Movement`)
      (:`Update`
        (`SceneComponent.K2_SetRelativeRotation` (`self.Lid`) (`KismetMathLibrary.MakeRotator` _open_angle) false false))
      (:`Finished`
        (set `self.IsOpen` true)))))

(fn `UserConstructionScript`)