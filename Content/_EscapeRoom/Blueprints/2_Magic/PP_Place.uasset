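; PP_Place is an escape room puzzle slot where the player places an item, counted as solved only for the Oktaerd class.
; Clicking the mesh runs the Item's used-item check, and hovering shows a hand cursor.
; Solve spawns and snaps the item onto the slot, signals success if correct, and clears the solved state when that item is destroyed.
; The construction script tints a dynamic outline material with the slot's Color.
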(event `self.PPMeshComponent.OnClicked`
  (params (TouchedComponent :type "PrimitiveComponent Object Reference") (ButtonPressed :type "Key Structure"))
  (`ItemComponent.CheckUsedItem` (`self.Item`))
  (set `PlayerController.CurrentMouseCursor` "Default" (`GameplayStatics.GetPlayerController` 0)))

(event `self.Solve`
  (bind _returnvalue (`|SpawnActorFromClass` (`ItemComponent.ItemClass` (`self.Item`)) (`KismetMathLibrary.MakeTransform` (0.0 0.0 0.0)) "AlwaysSpawn" "OverrideRootScale" null null))
  (`self.K2_AttachToActor` _returnvalue self "None" "SnapToTarget" "SnapToTarget" "KeepRelative" true)
  (add `self.OnDestroyed` _returnvalue (delegate `On Destroyed Item`))
  (if (== (`ItemComponent.ItemClass` (`self.Item`)) (`self.Oktaerd`))
    (set `self.bIsSolved` true)
    (`self.OnSolve`)
    (else
      (set `self.bIsSolved` false))))

(event `On Destroyed Item` :!signature `self.OnDestroyed`
  (params (DestroyedActor :type "Actor Object Reference"))
  (set `self.bIsSolved` false))

(event `self.PuzzlePartInteractCollision.OnEndCursorOver`
  (params (TouchedComponent :type "PrimitiveComponent Object Reference"))
  (set `PlayerController.CurrentMouseCursor` "Default" (`GameplayStatics.GetPlayerController` 0)))

(event `self.PuzzlePartInteractCollision.OnBeginCursorOver`
  (params (TouchedComponent :type "PrimitiveComponent Object Reference"))
  (set `PlayerController.CurrentMouseCursor` "Hand" (`GameplayStatics.GetPlayerController` 0)))

(fn `UserConstructionScript`
  (bind _ppmeshcomponent (`self.PPMeshComponent`))
  (bind _returnvalue (`PrimitiveComponent.CreateDynamicMaterialInstance` _ppmeshcomponent 0 "/Game/_EscapeRoom/Materials/Post_Process/M_Place_Outline.M_Place_Outline" "None"))
  (`MaterialInstanceDynamic.SetVectorParameterValue` _returnvalue "Colour" (`self.Color`))
  (`PrimitiveComponent.SetMaterial` _ppmeshcomponent 0 _returnvalue))