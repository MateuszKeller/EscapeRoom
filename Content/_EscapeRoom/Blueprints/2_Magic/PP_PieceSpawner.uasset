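; PP_PieceSpawner is a clickable spot in the Magic escape room that delivers gate puzzle pieces based on an item.
; Clicking its mesh asks the Item to check the used item and resets the mouse cursor to default.
; Solve matches the item name, Arch or Pillar, and moves the corresponding Gate child actor to the Gate's spawn point, printing an error for other names.
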(event `self.PPMeshComponent.OnClicked`
  (params (TouchedComponent :type "PrimitiveComponent Object Reference") (ButtonPressed :type "Key Structure"))
  (`ItemComponent.CheckUsedItem` (`self.Item`))
  (set `PlayerController.CurrentMouseCursor` "Default" (`GameplayStatics.GetPlayerController` 0)))

(event `self.Solve`
  (bind _gate (`self.Gate`))
  (bind _returnvalue (`SceneComponent.K2_GetComponentLocation` (`/Game/_EscapeRoom/Blueprints/2_Magic/PZ_Gate.Spawn` _gate)))
  (switch `string` (`KismetTextLibrary.Conv_TextToString` (`ItemComponent.ItemName` (`self.Item`)))
    (:`Default`
      (`KismetSystemLibrary.PrintString` "Wrong Item Name"))
    (:`Arch`
      (`self.K2_SetActorLocation` (`ChildActorComponent.ChildActor` (`/Game/_EscapeRoom/Blueprints/2_Magic/PZ_Gate.T4` _gate)) _returnvalue false false))
    (:`Pillar`
      (`self.K2_SetActorLocation` (`ChildActorComponent.ChildActor` (`/Game/_EscapeRoom/Blueprints/2_Magic/PZ_Gate.T5` _gate)) _returnvalue false false))))

(fn `UserConstructionScript`)