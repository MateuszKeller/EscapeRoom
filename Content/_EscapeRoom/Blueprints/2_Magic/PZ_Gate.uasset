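; Gate puzzle for the magic escape-room level, solved by mouse-dragging pieces until five child actors each sit wholly inside their matching trigger volume.
; A click line-traces for a movable component to drag, while Tick moves it and latches the solved flag.
; Releasing the mouse once solved hides the cursor, notifies the Answerer and changes view.
; A separate SmoothCameraMovement event turns the puzzle camera toward the Answerer before switching view.
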(event `self.ReceiveBeginPlay`)

(event `self.ReceiveTick`
  (params (DeltaSeconds :type "Float (single-precision)"))
  (`/Game/_EscapeRoom/Libraries/ActorLibrary.Drag Component with Mouse` (`self.Dragged Object`) (`self.Relative From Center`))
  (bind _returnvalue (`self.IsSolved`))
  (if _returnvalue
    (set `self.bIsSolved` true)))

(event `Key|LeftMouseButton`
  (params (Key :type "Key Structure"))
  (bind (_worldlocation _worlddirection) (`PlayerController.DeprojectMousePositionToWorld` (`GameplayStatics.GetPlayerController` 0)))
  (:`Pressed`
    (bind (_outhit _returnvalue) (`KismetSystemLibrary.LineTraceSingle` :`Start` _worldlocation :`End` (+ _worldlocation (* _worlddirection 200.0)) :`TraceChannel` "TraceTypeQuery1" :`bTraceComplex` true :`bIgnoreSelf` false))
    (if _returnvalue
      (if (`|EnumEquality` "Movable" (`SceneComponent.Mobility` (`.HitComponent` (`GameplayStatics.BreakHitResult` _outhit))))
        (set `self.Dragged Object` (`.HitComponent` (`GameplayStatics.BreakHitResult` _outhit)))
        (set `self.Relative From Center` (`KismetMathLibrary.InverseTransformLocation` (`KismetMathLibrary.Conv_VectorToTransform` (`SceneComponent.K2_GetComponentLocation` (`.HitComponent` (`GameplayStatics.BreakHitResult` _outhit)))) (`.Location` (`GameplayStatics.BreakHitResult` _outhit)))))))
  (:`Released`
    (set `self.Dragged Object` null)
    (if (`self.bIsSolved`)
      (`self.OnSolve`))))

(event `self.OnSolve`
  (set `PlayerController.bShowMouseCursor` false (`GameplayStatics.GetPlayerController` 0))
  (`PuzzleAnswerer.Answer` (`self.Answerer`))
  (`self.ChangeView`))

(event `Smooth Camera Movement`
  (bind _puzzlecamera (`self.PuzzleCamera`))
  (set `self.Gate Loc` (`SceneComponent.K2_GetComponentLocation` (`self.GetComponentByClass` (`self.Answerer`) "/Script/Engine.SceneComponent")))
  (set `self.Camera Loc` (`SceneComponent.K2_GetComponentLocation` _puzzlecamera))
  (set `self.Camera Rot` (`SceneComponent.K2_GetComponentRotation` _puzzlecamera))
  (bind (_direction _camera_to_gate) (`Timeline|Camera Rotation`)
    (:`Update`
      (`SceneComponent.K2_SetWorldRotation` (`self.PuzzleCamera`) (`KismetMathLibrary.RLerp` (`self.Camera Rot`) (`KismetMathLibrary.FindLookAtRotation` (`self.Camera Loc`) (`self.Gate Loc`)) _camera_to_gate true) false false))
    (:`Finished`
      (`Controller.SetControlRotation` (`GameplayStatics.GetPlayerController` 0) (`KismetMathLibrary.FindLookAtRotation` (`SceneComponent.K2_GetComponentLocation` (`self.GetComponentByClass` (`GameplayStatics.GetPlayerCharacter` 0) "/Script/Engine.CameraComponent")) (`self.Gate Loc`)))
      (`KismetSystemLibrary.Delay` 0.5)
      (`self.ChangeView`))))

(fn `IsSolved`
  (returns (ReturnValue :type Boolean))
  (bind _is_whole_inside (`/Game/_EscapeRoom/Libraries/ActorLibrary.Is Whole Actor Inside Volume` (`ChildActorComponent.ChildActor` (`self.T2`)) (`self.Trigger_2`)))
  (bind _is_whole_inside_2 (`/Game/_EscapeRoom/Libraries/ActorLibrary.Is Whole Actor Inside Volume` (`ChildActorComponent.ChildActor` (`self.T1`)) (`self.Trigger_1`)))
  (bind _is_whole_inside_3 (`/Game/_EscapeRoom/Libraries/ActorLibrary.Is Whole Actor Inside Volume` (`ChildActorComponent.ChildActor` (`self.T4`)) (`self.Trigger_4`)))
  (bind _is_whole_inside_4 (`/Game/_EscapeRoom/Libraries/ActorLibrary.Is Whole Actor Inside Volume` (`ChildActorComponent.ChildActor` (`self.T3`)) (`self.Trigger_3`)))
  (bind _is_whole_inside_5 (`/Game/_EscapeRoom/Libraries/ActorLibrary.Is Whole Actor Inside Volume` (`ChildActorComponent.ChildActor` (`self.T5`)) (`self.Trigger_5`)))
  (return (and _is_whole_inside _is_whole_inside_2 _is_whole_inside_3 _is_whole_inside_4 _is_whole_inside_5)))

(fn `UserConstructionScript`)