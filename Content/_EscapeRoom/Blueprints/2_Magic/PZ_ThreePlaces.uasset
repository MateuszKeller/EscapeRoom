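; PZ_ThreePlaces is an escape room puzzle actor that is solved once every place in its Places array is solved.
; It binds to each place's solve event on BeginPlay and rechecks all of them whenever one fires.
; When all are solved, it calls Answer on its Answerer and marks itself solved.
; Interacting while unsolved shows the player a message that more Octahedrons are needed.
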(event `self.ReceiveBeginPlay`
  (for _array_element (`self.Places`)
    (add `PuzzlePart.OnSolve` _array_element (delegate `Solve`))))

(event `Solve`
  (bind _returnvalue (`self.IsSolved`))
  (if _returnvalue
    (`self.OnSolve`)))

(event `self.OnInteract`
  (params (Player :type "PlayerCharacter Object Reference"))
  (if (not (`self.bIsSolved`))
    (`PlayerCharacter.OnMessageAnimation` Player "Need more Octahedrons" 2.0)))

(event `self.OnSolve`
  (`PuzzleAnswerer.Answer` (`self.Answerer`))
  (set `self.bIsSolved` true))

(fn `IsSolved`
  (returns (ReturnValue :type Boolean))
  (set `self.bIsSolved` true)
  (for _array_element (`self.Places`)
    (set `self.bIsSolved` (and (`PuzzlePart.bIsSolved` _array_element) (`self.bIsSolved`))))
  (return (`self.bIsSolved`)))

(fn `UserConstructionScript`)