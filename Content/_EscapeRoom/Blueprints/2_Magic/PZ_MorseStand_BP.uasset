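; Morse code puzzle stand for the escape room that signals "HASTUR" with a spotlight and beeps; solving it notifies an Answerer.
; Interacting switches the view, then clicking the disc in the Puzzle state spins it and starts playback.
; Repeat sequences a red start flash and per-letter MultiGate events using hand-tuned delays, with DotDash and BeepGap timing each pulse from sound duration.
; DotDash stops the signal if the player leaves the Puzzle state.
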(event `self.ReceiveBeginPlay`
  (`self.Reset Light`))

(event `self.ReceiveTick`
  (params (DeltaSeconds :type "Float (single-precision)"))
  (if (`self.is Disc Rotating`)
    (`SceneComponent.K2_AddLocalRotation` (`self.Disc`) (struct :`Yaw` 1.0) false false)))

(event `self.OnInteract`
  (params (Player :type "PlayerCharacter Object Reference"))
  (if (`self.bIsSolved`)
    _
    (elif (`self.bHasStoppedPlaying`)
      (`PlayerCharacter.OnPointerTextUpdate` Player "")
      (`Interactable.OnStopLooking`)
      (`self.ChangeView`))))

(event `self.OnSolve`
  (`PuzzleAnswerer.Answer` (`self.Answerer`))
  (`self.ChangeView`))

(event `self.Disc.OnClicked`
  (params (TouchedComponent :type "PrimitiveComponent Object Reference") (ButtonPressed :type "Key Structure"))
  (bind _is_correct (`/Game/_EscapeRoom/Libraries/HUDFormatingLibrary.ComparePlayerState` "Puzzle"))
  (if _is_correct
    (if (`self.bHasStoppedPlaying`)
      (set `self.is Disc Rotating` true)
      (`self.Start Signal`)
      (set `PlayerController.CurrentMouseCursor` "Default" (`GameplayStatics.GetPlayerController` 0)))))

(event `self.Disc.OnBeginCursorOver`
  (params (TouchedComponent :type "PrimitiveComponent Object Reference"))
  (set `PlayerController.CurrentMouseCursor` "Hand" (`GameplayStatics.GetPlayerController` 0)))

(event `self.Disc.OnEndCursorOver`
  (params (TouchedComponent :type "PrimitiveComponent Object Reference"))
  (set `PlayerController.CurrentMouseCursor` "Default" (`GameplayStatics.GetPlayerController` 0)))

(event `H`
  (bind _dot_sound (`self.Dot Sound`))
  (if (`self.Does Play Morse`)
    (`|MultiGate` false :!label _label
      (:`Out 0`
        (bind _duration (`self.Dot Dash` _dot_sound))
        (`self.Beep Gap` _duration
          (:`End`
            _)))
      (:`Out 1`
        (bind _duration_2 (`self.Dot Dash` _dot_sound))
        (`self.Beep Gap` _duration_2
          (:`End`
            _)))
      (:`Out 2`
        (bind _duration_3 (`self.Dot Dash` _dot_sound))
        (`self.Beep Gap` _duration_3
          (:`End`
            _)))
      (:`Out 3`
        (bind _duration_4 (`self.Dot Dash` _dot_sound))
        (`self.Beep Gap` _duration_4
          (:`End`
            (`KismetSystemLibrary.Delay` 0.7)
            (goto _label :!via `Reset`)))))
    (`self.H`)
    (else
      (goto _label :!via `Reset`))))

(event `Start Signal`
  (set `self.Does Play Morse` true)
  (set `self.bHasStoppedPlaying` false)
  (`self.Repeat`))

(event `A`
  (if (`self.Does Play Morse`)
    (`|MultiGate` false :!label _label_2
      (:`Out 0`
        (bind _duration (`self.Dot Dash` (`self.Dot Sound`)))
        (`self.Beep Gap` _duration
          (:`End`
            (`self.A`))))
      (:`Out 1`
        (bind _duration_2 (`self.Dot Dash` (`self.Dash Sound`)))
        (`self.Beep Gap` _duration_2
          (:`End`
            (`KismetSystemLibrary.Delay` 0.7)
            (goto _label_2 :!via `Reset`)))))
    (else
      (goto _label_2 :!via `Reset`))))

(event `Repeat`
  (if (`self.Does Play Morse`)
    (`|MultiGate` false true :!label _label_3
      (:`Out 0`
        (`self.End Start`)
        (`KismetSystemLibrary.Delay` 1.5)
        (`self.Repeat` :!label _label_4))
      (:`Out 1`
        (`self.h`)
        (`KismetSystemLibrary.Delay` 3.06)
        (goto _label_4))
      (:`Out 2`
        (`self.a`)
        (`KismetSystemLibrary.Delay` 2.36)
        (goto _label_4))
      (:`Out 3`
        (`self.S`)
        (`KismetSystemLibrary.Delay` 2.47)
        (goto _label_4))
      (:`Out 4`
        (`self.T`)
        (`KismetSystemLibrary.Delay` 1.77)
        (goto _label_4))
      (:`Out 5`
        (`self.U`)
        (`KismetSystemLibrary.Delay` 2.95)
        (goto _label_4))
      (:`Out 6`
        (`self.R`)
        (`KismetSystemLibrary.Delay` 2.95)
        (`self.Reset Playing`)))
    (else
      (`self.Reset Light`)
      (goto _label_3 :!via `Reset`))))

(event `S`
  (bind _dot_sound (`self.Dot Sound`))
  (if (`self.Does Play Morse`)
    (`|MultiGate` false :!label _label_5
      (:`Out 0`
        (bind _duration (`self.Dot Dash` _dot_sound))
        (`self.Beep Gap` _duration
          (:`End`
            _)))
      (:`Out 1`
        (bind _duration_2 (`self.Dot Dash` _dot_sound))
        (`self.Beep Gap` _duration_2
          (:`End`
            _)))
      (:`Out 2`
        (bind _duration_3 (`self.Dot Dash` _dot_sound))
        (`self.Beep Gap` _duration_3
          (:`End`
            (`KismetSystemLibrary.Delay` 0.7)
            (goto _label_5 :!via `Reset`)))))
    (`self.S`)
    (else
      (goto _label_5 :!via `Reset`))))

(event `T`
  (if (`self.Does Play Morse`)
    (bind _duration (`self.Dot Dash` (`self.Dash Sound`)))
    (`self.Beep Gap` _duration
      (:`End`
        (`KismetSystemLibrary.Delay` 0.7)))))

(event `End Start`
  (bind _spotlight (`self.SpotLight`))
  (`LightComponent.SetLightColor` _spotlight (struct :`R` 1.0 :`A` 1.0) true)
  (`SceneComponent.SetVisibility` _spotlight true false)
  (`KismetSystemLibrary.Delay` 1.5)
  (`LightComponent.SetLightColor` _spotlight (struct :`R` 1.0 :`G` 1.0 :`B` 1.0 :`A` 1.0) true)
  (`SceneComponent.SetVisibility` _spotlight false false))

(event `U`
  (if (`self.Does Play Morse`)
    (`|MultiGate` false :!label _label_6
      (:`Out 0`
        (bind _duration (`self.Dot Dash` (`self.Dot Sound`)))
        (`self.Beep Gap` _duration
          (:`End`
            _)))
      (:`Out 1`
        (bind _duration_2 (`self.Dot Dash` (`self.Dot Sound`)))
        (`self.Beep Gap` _duration_2
          (:`End`
            _)))
      (:`Out 2`
        (bind _duration_3 (`self.Dot Dash` (`self.Dash Sound`)))
        (`self.Beep Gap` _duration_3
          (:`End`
            (`KismetSystemLibrary.Delay` 0.7)
            (goto _label_6 :!via `Reset`)))))
    (`self.U`)
    (else
      (goto _label_6 :!via `Reset`))))

(event `Reset Light`
  (bind _spotlight (`self.SpotLight`))
  (`LightComponent.SetLightColor` _spotlight (struct :`R` 1.0 :`A` 1.0) true)
  (`SceneComponent.SetVisibility` _spotlight false false)
  (set `self.bHasStoppedPlaying` true)
  (set `self.is Disc Rotating` false))

(event `R`
  (if (`self.Does Play Morse`)
    (`|MultiGate` false :!label _label_7
      (:`Out 0`
        (bind _duration (`self.Dot Dash` (`self.Dot Sound`)))
        (`self.Beep Gap` _duration
          (:`End`
            _)))
      (:`Out 1`
        (bind _duration_2 (`self.Dot Dash` (`self.Dash Sound`)))
        (`self.Beep Gap` _duration_2
          (:`End`
            _)))
      (:`Out 2`
        (bind _duration_3 (`self.Dot Dash` (`self.Dot Sound`)))
        (`self.Beep Gap` _duration_3
          (:`End`
            (`KismetSystemLibrary.Delay` 0.7)
            (goto _label_7 :!via `Reset`)))))
    (`self.R`)
    (else
      (goto _label_7 :!via `Reset`))))

(fn `Check if still plating`
  (returns (`Does Play Morse` :type Boolean))
  (bind _is_correct (`/Game/_EscapeRoom/Libraries/HUDFormatingLibrary.ComparePlayerState` "Puzzle"))
  (if (not _is_correct)
    (set `self.Does Play Morse` false))
  (return (`self.Does Play Morse`)))

(fn `Dot Dash`
  (params (Sound :type "SoundBase Object Reference"))
  (returns (Duration :type "Float (double-precision)"))
  (bind _does_play_morse (`self.Check if still plating`))
  (if _does_play_morse
    (`|ExecutionSequence`
      (:`then_0`
        (`SceneComponent.SetVisibility` (`self.SpotLight`) true false))
      (:`then_1`
        (`GameplayStatics.PlaySoundAtLocation` Sound (`SceneComponent.K2_GetComponentLocation` (`self.Speaker`)) (struct) 1.0 1.0 0.0 "/Game/_EscapeRoom/Audio/BeepFalloff.BeepFalloff" null null)
        (return (`SoundBase.Duration` Sound))))
    (else
      (return 0.0))))

(fn `Reset Playing`
  (set `self.is Disc Rotating` false)
  (set `self.bHasStoppedPlaying` true))

(fn `UserConstructionScript`)