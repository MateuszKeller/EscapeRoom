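; DummyItem is an escape room actor that displays a stand-in mesh for a given item and signals mouse interactivity.
; CorrectMesh configures it from the passed Item, copying its dummy mesh, relative scale and name.
; Mesh cursor events switch the player's cursor to a hand on hover and back to default when hover ends or a click is released.
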(event `self.StaticMeshComponent.OnBeginCursorOver`
  (params (TouchedComponent :type "PrimitiveComponent Object Reference"))
  (set `PlayerController.CurrentMouseCursor` "Hand" (`GameplayStatics.GetPlayerController` 0)))

(event `self.StaticMeshComponent.OnEndCursorOver`
  (params (TouchedComponent :type "PrimitiveComponent Object Reference"))
  (set `PlayerController.CurrentMouseCursor` "Default" (`GameplayStatics.GetPlayerController` 0)))

(event `self.StaticMeshComponent.OnReleased`
  (params (TouchedComponent :type "PrimitiveComponent Object Reference") (ButtonReleased :type "Key Structure"))
  (set `PlayerController.CurrentMouseCursor` "Default" (`GameplayStatics.GetPlayerController` 0)))

(fn `Correct Mesh`
  (params (Item :type "ItemComponent Object Reference"))
  (bind _staticmeshcomponent (`self.StaticMeshComponent`))
  (`StaticMeshComponent.SetStaticMesh` _staticmeshcomponent (`ItemComponent.DummyMesh` Item))
  (`SceneComponent.SetRelativeScale3D` _staticmeshcomponent (`ItemComponent.Scale` Item))
  (set `self.Name` (`ItemComponent.ItemName` Item)))

(fn `UserConstructionScript`)